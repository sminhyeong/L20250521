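; BP_P38 is a player-controlled P-38 plane that constantly moves along its forward vector.
; Roll and Pitch axes rotate it locally, and holding the boost input doubles its speed rate.
; Attack spawns a BP_Rocket at the plane's transform, then a Tick-driven countdown blocks firing until the cooldown resets.
; BeginPlay registers the Left and Right components with BPSceneRotator, presumably to spin them.
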(event EventBeginPlay
  (Variables|Default|SetSpeedRate (Variables|Default|GetDefaultSpeedRate))
  (Variables|Default|SetCurCoolTime (Variables|Default|GetDefaultCoolTime))
  (Default|AddComponent (Variables|Default|GetBP_SceneRotator) (Variables|Default|GetLeft))
  (Default|AddComponent (Variables|Default|GetBP_SceneRotator) (Variables|Default|GetRight)))

(event EventTick
  (params (DeltaSeconds :type Float%20%28single-precision%29))
  (Pawn|Input|AddMovementInput (Transformation|GetActorForwardVector) (Variables|Default|GetSpeedRate) false)
  (if (< (Variables|Default|GetCurCoolTime) (Variables|Default|GetDefaultCoolTime))
    (Variables|Default|SetCurCoolTime (- (Variables|Default|GetCurCoolTime) (Utilities|Time|GetWorldDeltaSeconds)))
    (if (<= (Variables|Default|GetCurCoolTime) 0.0)
      (Variables|Default|SetCurCoolTime (Variables|Default|GetDefaultCoolTime)))))

(event Input|ActionEvents|InputActionAttack
  (params (Key :type Key%20Structure :default "None"))
  (:Pressed
    (if (>= (Variables|Default|GetCurCoolTime) (Variables|Default|GetDefaultCoolTime))
      (Game|SpawnActorfromClass "/Game/Blueprint/BP_Rocket.BP_Rocket_C" (Transformation|GetActorTransform) "Undefined" "MultiplyWithRoot" 0 0)
      (Variables|Default|SetCurCoolTime (- (Variables|Default|GetCurCoolTime) (Utilities|Time|GetWorldDeltaSeconds))))))

(event Input|ActionEvents|InputActionBosst
  (params (Key :type Key%20Structure :default "None"))
  (:Pressed
    (Variables|Default|SetSpeedRate (* (Variables|Default|GetDefaultSpeedRate) 2.0)))
  (:Released
    (Variables|Default|SetSpeedRate (Variables|Default|GetDefaultSpeedRate))))

(event Input|AxisEvents|InputAxisRoll
  (params (AxisValue :type Float%20%28single-precision%29))
  (Transformation|AddActorLocalRotation (Math|Rotator|MakeRotator (* AxisValue (Utilities|Time|GetWorldDeltaSeconds) (Variables|Default|GetRotateRate)) 0.0 0.0) false false))

(event Input|AxisEvents|InputAxisPitch
  (params (AxisValue :type Float%20%28single-precision%29))
  (Transformation|AddActorLocalRotation (Math|Rotator|MakeRotator 0.0 (* AxisValue (Utilities|Time|GetWorldDeltaSeconds) (Variables|Default|GetRotateRate)) 0.0) false false))

(fn ConstructionScript)